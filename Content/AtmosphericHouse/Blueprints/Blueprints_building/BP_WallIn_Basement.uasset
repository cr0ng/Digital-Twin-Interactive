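; Modular basement interior wall piece for the Atmospheric House building set, configured entirely in the construction script.
; The WallInBasement enum picks the wall, column or corner mesh from an array.
; Optional toggles add a doorframe child actor on door variants and a matching corner decal mesh on columns and small/large outer corners, destroying the decal component otherwise.
; A self-resetting RevertDefaultMaterials toggle restores the mesh's default materials.
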(event EventBeginPlay)

(event Collision|EventActorBeginOverlap
  (params (OtherActor :type Actor%20Object%20Reference)))

(event EventTick
  (params (DeltaSeconds :type Float%20%28single-precision%29)))

(fn ConstructionScript
  (bind _returnvalue (Math|Transform|MakeTransform "0,-150.000000,0.000000"))
  (bind _wallin_c_mesh (Variables|Default|GetWallIn_C_mesh))
  ;[1 1 1] WallIn Mesh Assign
  (Components|StaticMesh|SetStaticMesh (Variables|Default|GetWallIn_C_mesh) (Utilities|Array|Get(acopy) (Variables|Mesh|GetWall%20in%20C%20Meshes) (Math|Conversions|ToInteger(Byte) (Variables|Mesh|GetWallIn_Basement))))
  ;[1 1 1] Doorframe
  (if (Variables|Mesh|GetDoorframe)
    (switch Utilities|FlowControl|Switch|SwitchonE_WallIn_Basement (Variables|Mesh|GetWallIn_Basement)
      (:NewEnumerator19
        _)
      (:NewEnumerator25
        _)
      (:NewEnumerator43
        _)
      (:NewEnumerator44
        (AddComponent|AddChildActorComponent false _returnvalue))
      (:NewEnumerator45
        (AddComponent|AddChildActorComponent false _returnvalue))
      (:NewEnumerator46
        _)
      (:NewEnumerator47
        _)
      (:NewEnumerator48
        _)
      (:NewEnumerator49
        _)
      (:NewEnumerator50
        _)
      (:NewEnumerator51
        _)
      (:NewEnumerator54
        _)
      (:NewEnumerator55
        _)
      (:NewEnumerator56
        _)
      (:NewEnumerator57
        _)))
  ;[1 1 1] Corner Decals
  (if (Variables|Mesh|GetDecal_corner)
    (if true
      (switch Utilities|FlowControl|Switch|SwitchonE_WallIn_Basement (Variables|Mesh|GetWallIn_Basement)
        (:NewEnumerator19
          (Components|DestroyComponent (Variables|Default|GetDecal_corner_mesh) :!label _label))
        (:NewEnumerator25
          (goto _label))
        (:NewEnumerator43
          (goto _label))
        (:NewEnumerator44
          (goto _label))
        (:NewEnumerator45
          (goto _label))
        (:NewEnumerator46
          (goto _label))
        (:NewEnumerator47
          (Components|StaticMesh|SetStaticMesh (Variables|Default|GetDecal_corner_mesh) (Utilities|Array|Get(acopy) (Variables|Mesh|GetDecal%20Corner%20C%20Meshes) (Math|Conversions|ToInteger(Byte) (Variables|Mesh|GetWallIn_Basement))) :!label _label_2))
        (:NewEnumerator48
          (goto _label_2))
        (:NewEnumerator49
          (goto _label_2))
        (:NewEnumerator50
          (goto _label_2))
        (:NewEnumerator51
          (goto _label_2))
        (:NewEnumerator54
          (goto _label_2))
        (:NewEnumerator55
          (goto _label_2))
        (:NewEnumerator56
          (goto _label))
        (:NewEnumerator57
          (goto _label)))
      (else
        (goto _label)))
    (else
      (goto _label)))
  ;[1 1 1] Revert Materials
  (if (Variables|Mesh|GetRevert%20Default%20Materials)
    (bind _output_get (LocalVariables|SetNumber%20Of%20Materials (Rendering|Material|GetNumMaterials _wallin_c_mesh)))
    (for _index (range 0 _output_get)
      (Rendering|Material|SetMaterial _wallin_c_mesh _index (Rendering|Material|GetMaterial (Variables|/Script/Engine.StaticMeshComponent|GetStaticMesh _wallin_c_mesh) _index)))
    (Variables|Mesh|SetRevert%20Default%20Materials false)))