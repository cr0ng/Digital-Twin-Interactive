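; Master door Blueprint for the atmospheric house that builds a posed door at edit time, with no runtime logic.
; The construction script switches on the Doors type to spawn child actor components: left or right single, double in A/B/C styles, or sliding pair.
; OnewayDoor selects hinge offsets and the yaw variable, mirrored for right-hand leaves.
; Sliding leaves ignore that choice, mapping SlidingDoorL and SlidingDoorR to clamped Y offsets.
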(event EventBeginPlay)

(event Collision|EventActorBeginOverlap
  (params (OtherActor :type Actor%20Object%20Reference)))

(event EventTick
  (params (DeltaSeconds :type Float%20%28single-precision%29)))

(fn ConstructionScript
  (bind _door_rotation_multiway (Variables|Mesh|GetDoor%20Rotation%20Multiway))
  (bind _door_rotation_oneway (Variables|Mesh|GetDoor%20Rotation%20Oneway))
  (bind _door_rotation_oneway_2 (Variables|Mesh|GetDoor%20Rotation%20Oneway))
  (bind _door_rotation_multiway_2 (Variables|Mesh|GetDoor%20Rotation%20Multiway))
  (bind _returnvalue (Math|Rotator|MakeRotator 0.0 0.0 _door_rotation_oneway))
  (bind _returnvalue_2 (Math|Rotator|MakeRotator 0.0 0.0 _door_rotation_multiway_2))
  (bind _returnvalue_3 (Math|Rotator|MakeRotator 0.0 0.0 _door_rotation_multiway))
  (bind _returnvalue_4 (Math|Rotator|MakeRotator 0.0 0.0 _door_rotation_oneway_2))
  (bind _returnvalue_5 (* _door_rotation_oneway_2 -1.0))
  (bind _returnvalue_6 (* _door_rotation_multiway -1.0))
  (bind _returnvalue_7 (Math|Rotator|MakeRotator 0.0 0.0 _returnvalue_5))
  (bind _returnvalue_8 (Math|Transform|MakeTransform "0,-98.449997, 0" _returnvalue_3))
  (bind _returnvalue_9 (Math|Rotator|MakeRotator 0.0 0.0 _returnvalue_6))
  (bind _returnvalue_10 (Math|Transform|MakeTransform "-14.000000,-1.500000, 0" _returnvalue))
  (bind _returnvalue_11 (Class|KismetMathLibrary|NegateRotator _returnvalue_2))
  (bind _returnvalue_12 (Class|KismetMathLibrary|NegateRotator _returnvalue))
  (bind _returnvalue_13 (Math|Transform|MakeTransform "0,2.000000, 0" _returnvalue_2))
  (bind _returnvalue_14 (Math|Transform|MakeTransform "-14.000000,-103.099998, 0" _returnvalue_4))
  (bind _returnvalue_15 (Math|Transform|MakeTransform "0,98.449997, 0" _returnvalue_9))
  (bind _returnvalue_16 (Math|Transform|MakeTransform "-14.000000,101.500000, 0" _returnvalue_12))
  (bind _returnvalue_17 (Math|Transform|MakeTransform "0.000000,98.000000, 0" _returnvalue_11))
  (bind _returnvalue_18 (Math|Transform|MakeTransform "-14.000000,103.099998, 0" _returnvalue_7))
  (if (Variables|Mesh|GetOneway%20Door?)
    (switch Utilities|FlowControl|Switch|SwitchonE_Doors (Variables|Mesh|GetDoors)
      (:NewEnumerator19
        (AddComponent|AddChildActorComponent false _returnvalue_10))
      (:NewEnumerator43
        (AddComponent|AddChildActorComponent false _returnvalue_10))
      (:NewEnumerator45
        (AddComponent|AddChildActorComponent false _returnvalue_10))
      (:NewEnumerator51
        (AddComponent|AddChildActorComponent false _returnvalue_16))
      (:NewEnumerator52
        (AddComponent|AddChildActorComponent false _returnvalue_16))
      (:NewEnumerator53
        (AddComponent|AddChildActorComponent false _returnvalue_16))
      (:NewEnumerator47
        (AddComponent|AddChildActorComponent false _returnvalue_14)
        (AddComponent|AddChildActorComponent false _returnvalue_18))
      (:NewEnumerator48
        (AddComponent|AddChildActorComponent false _returnvalue_14)
        (AddComponent|AddChildActorComponent false _returnvalue_18))
      (:NewEnumerator49
        (AddComponent|AddChildActorComponent false _returnvalue_14)
        (AddComponent|AddChildActorComponent false _returnvalue_18))
      (:NewEnumerator50
        (AddComponent|AddChildActorComponent false (Math|Transform|MakeTransform (Math|Vector|MakeVector 0.0 (Math|Float|MapRangeClamped (Variables|Mesh|GetSliding%20Door%20L) 0.0 1.0 1.0 99.0) 0.0)))
        (AddComponent|AddChildActorComponent false (Math|Transform|MakeTransform (Math|Vector|MakeVector 0.0 (* (Math|Float|MapRangeClamped (Variables|Mesh|GetSliding%20Door%20R) 0.0 1.0 1.0 99.0) -1.0) 0.0) "0,180.000000, 0"))))
    (else
      (switch Utilities|FlowControl|Switch|SwitchonE_Doors (Variables|Mesh|GetDoors)
        (:NewEnumerator19
          (AddComponent|AddChildActorComponent false _returnvalue_13))
        (:NewEnumerator43
          (AddComponent|AddChildActorComponent false _returnvalue_13))
        (:NewEnumerator45
          (AddComponent|AddChildActorComponent false _returnvalue_13))
        (:NewEnumerator51
          (AddComponent|AddChildActorComponent false _returnvalue_17))
        (:NewEnumerator52
          (AddComponent|AddChildActorComponent false _returnvalue_17))
        (:NewEnumerator53
          (AddComponent|AddChildActorComponent false _returnvalue_17))
        (:NewEnumerator47
          (AddComponent|AddChildActorComponent false _returnvalue_8)
          (AddComponent|AddChildActorComponent false _returnvalue_15))
        (:NewEnumerator48
          (AddComponent|AddChildActorComponent false _returnvalue_8)
          (AddComponent|AddChildActorComponent false _returnvalue_15))
        (:NewEnumerator49
          (AddComponent|AddChildActorComponent false _returnvalue_8)
          (AddComponent|AddChildActorComponent false _returnvalue_15))
        (:NewEnumerator50
          (AddComponent|AddChildActorComponent false (Math|Transform|MakeTransform (Math|Vector|MakeVector 0.0 (Math|Float|MapRangeClamped (Variables|Mesh|GetSliding%20Door%20L) 0.0 1.0 1.0 99.0) 0.0)))
          (AddComponent|AddChildActorComponent false (Math|Transform|MakeTransform (Math|Vector|MakeVector 0.0 (* (Math|Float|MapRangeClamped (Variables|Mesh|GetSliding%20Door%20R) 0.0 1.0 1.0 99.0) -1.0) 0.0) "0,180.000000, 0")))))))